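; BP_HealthRegen is a health pickup with a spinning cross that respawns after being consumed.
; On overlap, it asks the other actor's BP_HealthComp to regenerate a random amount of health and is consumed only if that call returns true.
; Consumption hides the cross, disables trigger collision and attaches a green Niagara zap effect to the consumer, then restores the pickup after a delay.
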(event Custom|Consumed
  (params (ConsumedBy :type Actor%20Object%20Reference))
  (Rendering|SetVisibility (Variables|Default|GetCross) false true)
  (Collision|SetCollisionEnabled (Variables|Default|GetTrigger) "NoCollision")
  (Niagara|SpawnSystemAttached "/Game/Vefects/Zap_VFX/VFX/Zap/Particles/NS_Zap_04_Green.NS_Zap_04_Green" (Variables|/Script/Engine.Actor|GetRootComponent ConsumedBy) "None" "0, 0, 0" "0, 0, 0" "KeepRelativeOffset" false)
  (Utilities|FlowControl|Delay 1e+01)
  (Rendering|SetVisibility (Variables|Default|GetCross) true true)
  (Collision|SetCollisionEnabled (Variables|Default|GetTrigger) "QueryAndPhysics"))

(event EventBeginPlay
  (|CallParentFunction) ; This node is disabled and will not be called.\nDrag off pins to build functionality.
)

(event Collision|EventActorBeginOverlap
  (params (OtherActor :type Actor%20Object%20Reference))
  (|CallParentFunction OtherActor) ; This node is disabled and will not be called.\nDrag off pins to build functionality.
)

(event EventTick
  (params (DeltaSeconds :type Float%20%28single-precision%29))
  (|CallParentFunction DeltaSeconds)
  (Transformation|AddRelativeRotation (Variables|Default|GetCross) (Math|Rotator|MakeRotator 0.0 0.0 (* DeltaSeconds 1e+02)) false false))

(event EventOverlapped
  (params (OtherActor :type Actor%20Object%20Reference))
  (bind _regensuccessful (Default|RegenerateHealth (Actor|GetComponentbyClass OtherActor "/Game/Components/BP_HealthComp.BP_HealthComp_C") (Math|Random|RandomFloatinRange 1e+01 5e+01)))
  (if _regensuccessful
    (CallFunction|Consumed OtherActor)))

(fn ConstructionScript
  (|CallParentFunction))