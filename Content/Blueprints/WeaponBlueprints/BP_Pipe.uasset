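; BP_Pipe is a pipe weapon actor that damages pawns around it.
; Its only active logic is a custom event that runs a sphere overlap at the actor's location, sized by DamageRange and ignoring the owner.
; Each pawn found takes Damage, with the pipe as damage causer.
; Nothing in this Blueprint calls the event, and its BeginPlay, Tick and overlap events are disabled stubs.
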(event Custom|CustomEvent
  (bind _outactors (Collision|SphereOverlapActors (Transformation|GetActorLocation) (Variables|Default|GetDamageRange) (Utilities|Array|MakeArray "ObjectTypeQuery3") 0 (Utilities|Array|MakeArray (Components|GetOwner))))
  (for _array_element _outactors
    (Game|Damage|ApplyDamage _array_element (Variables|Default|GetDamage) 0 self)))

(event EventBeginPlay
  (|CallParentFunction) ; This node is disabled and will not be called.\nDrag off pins to build functionality.
)

(event Collision|EventActorBeginOverlap
  (params (OtherActor :type Actor%20Object%20Reference))
  (|CallParentFunction OtherActor) ; This node is disabled and will not be called.\nDrag off pins to build functionality.
)

(event EventTick
  (params (DeltaSeconds :type Float%20%28single-precision%29))
  (|CallParentFunction DeltaSeconds) ; This node is disabled and will not be called.\nDrag off pins to build functionality.
)

(fn ConstructionScript
  (|CallParentFunction))